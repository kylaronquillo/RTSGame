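; Player controller for the RTS game that pans the controlled camera pawn with movement input axes or mouse edge scrolling.
; The MouseMovement axis event sets forward and right scales whenever the cursor enters a threshold band at the viewport edges.
; The MoveForward and MoveRight events move the pawn along control-yaw directions, using the axis value when non-zero and falling back to those edge scales otherwise.
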(event EventBeginPlay)

(event EventTick
  (params (DeltaSeconds :type Float%20%28single-precision%29)))

(event Input|AxisEvents|InputAxisMoveForward
  (params (AxisValue :type Float%20%28single-precision%29))
  ;[1 1 1] Camera Movement
  (Pawn|Input|AddMovementInput (Pawn|GetControlledPawn) (Math|Vector|GetForwardVector (Math|Rotator|MakeRotator 0.0 0.0 (.yaw (Pawn|GetControlRotation :!class /Script/Engine.Controller)))) (Math|Float|SelectFloat AxisValue (Variables|Default|GetMouseForwardScale) (!= AxisValue 0.0)) false))

(event Input|AxisEvents|InputAxisMoveRIght
  (params (AxisValue :type Float%20%28single-precision%29))
  ;[1 1 1] Camera Movement
  (Pawn|Input|AddMovementInput (Pawn|GetControlledPawn) (Math|Vector|GetRightVector (Math|Rotator|MakeRotator 0.0 0.0 (.yaw (Pawn|GetControlRotation :!class /Script/Engine.Controller)))) (Math|Float|SelectFloat AxisValue (Variables|Default|GetMouseRightScale) (!= AxisValue 0.0)) false))

(event Input|AxisEvents|InputAxisMouseMovement
  (params (AxisValue :type Float%20%28single-precision%29))
  (bind _locationy (Game|Player|GetMousePosition))
  (bind _returnvalue (Viewport|GetViewportSize))
  (bind _locationx (Game|Player|GetMousePosition))
  (bind _returnvalue_2 (Viewport|GetViewportSize))
  (bind _returnvalue_3 (/ _locationx (.x _returnvalue_2)))
  (bind _returnvalue_4 (/ _locationy (.y _returnvalue)))
  ;[1 1 1] Camera Movement
  (Variables|Default|SetMouseRightScale (Math|Float|SelectFloat -1.0 (Math|Float|SelectFloat 1.0 0.0 (> _returnvalue_3 (- 1.0 (Variables|Default|GetViewport%20Edge%20Thresh)))) (< _returnvalue_3 (Variables|Default|GetViewport%20Edge%20Thresh))))
  (Variables|Default|SetMouseForwardScale (Math|Float|SelectFloat 1.0 (Math|Float|SelectFloat -1.0 0.0 (> _returnvalue_4 (- 1.0 (Variables|Default|GetViewport%20Edge%20Thresh)))) (< _returnvalue_4 (Variables|Default|GetViewport%20Edge%20Thresh)))))

(fn ConstructionScript)