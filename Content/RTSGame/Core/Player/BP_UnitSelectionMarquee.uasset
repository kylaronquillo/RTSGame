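; BP_UnitSelectionMarquee is a world-space marquee actor for RTS drag selection, anchored at its own location.
; While resizing, toggled by StartResizingMarquee and EndResizingMarquee, Tick traces under the cursor, moves Sphere there, and centers BoxCollision and Sphere2 midway to it.
; The box's X/Y extents span the two corners with fixed height.
; Overlapping actors implementing BPI_SelectionEvents are sent to the player controller for selection, with no end-overlap handling.
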(event OnComponentBeginOverlap(BoxCollision)
  (params (OverlappedComponent :type Primitive%20Component%20Object%20Reference) (OtherActor :type Actor%20Object%20Reference) (OtherComp :type Primitive%20Component%20Object%20Reference) (OtherBodyIndex :type Integer) (bFromSweep :type Boolean) (SweepResult :type Hit%20Result%20Structure%20%28by%20ref%29))
  (if (Utilities|DoesObjectImplementInterface OtherActor "/Game/RTSGame/Core/Building/BPI_SelectionEvents.BPI_SelectionEvents_C")
    (Class|BPISelectionEvents|SelectThisActor(Message) (Game|GetPlayerController 0) OtherActor)))

(event EventBeginPlay)

(event Collision|EventActorBeginOverlap
  (params (OtherActor :type Actor%20Object%20Reference)))

(event EventTick
  (params (DeltaSeconds :type Float%20%28single-precision%29))
  (if (Variables|Default|GetShouldResizeMarquee)
    (bind _aspc_rtsgame (Utilities|Casting|CastToPC_RTSGame (Game|GetPlayerController 0)))
    (Transformation|SetWorldLocation (Variables|Default|GetSphere) (.Location (Collision|BreakHitResult (.HitResult (Game|Player|GetHitResultUnderCursorbyChannel _aspc_rtsgame "TraceTypeQuery1" true)))) false false)
    (Variables|Default|SetEnd%20Mouse%20location (.Location (Collision|BreakHitResult (.HitResult (Game|Player|GetHitResultUnderCursorbyChannel _aspc_rtsgame "TraceTypeQuery1" true)))))
    (Transformation|SetWorldLocation (Variables|Default|GetBoxCollision) (Math|Vector|Lerp(Vector) (Transformation|GetActorLocation) (Variables|Default|GetEnd%20Mouse%20location) 0.5) false false)
    (Components|Box|SetBoxExtent (Variables|Default|GetBoxCollision) (Math|Vector|MakeVector (.x (/ (Math|Vector|VectorGetAbs (- (Transformation|GetActorLocation) (Variables|Default|GetEnd%20Mouse%20location))) 2.0)) (.y (/ (Math|Vector|VectorGetAbs (- (Transformation|GetActorLocation) (Variables|Default|GetEnd%20Mouse%20location))) 2.0)) 3e+02) true)))

(fn ConstructionScript)

(fn StartResizingMarquee
  (Variables|Default|SetShouldResizeMarquee true))

(fn EndResizingMarquee
  (Variables|Default|SetShouldResizeMarquee false))