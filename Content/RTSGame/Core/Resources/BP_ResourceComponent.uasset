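; BP_ResourceComponent is an RTS actor component that makes its owner a gatherable resource with a type, a yield per gather and a limited number of uses.
; GiveResource decrements the remaining uses, fires the gathered event, fires the exhausted event when none remain, then returns the type and amount.
; CanThisResourceBeMined reports whether uses remain, but GiveResource only checks it after decrementing, so it does not itself block gathering from a depleted resource.
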(event EventBeginPlay)

(event EventTick
  (params (DeltaSeconds :type Float%20%28single-precision%29)))

(fn GiveResource
  (Variables|Default|SetTimesCanBeMined (- (Variables|Default|GetTimesCanBeMined) 1))
  (Default|CallOnResourceGathered)
  (Utilities|FlowControl|Sequence
    (:then_0
      (if (not (CallFunction|CanThisResourcebeMined))
        (Default|CallOnResourceExhausted)))
    (:then_1
      (return (Variables|Default|GetTypeOfResource) (Variables|Default|GetNumOfResourcesToGive)))))

(fn CanThisResourcebeMined
  (return (> (Variables|Default|GetTimesCanBeMined) 0)))