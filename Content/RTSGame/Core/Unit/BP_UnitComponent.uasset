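; BP_UnitComponent is an actor component that makes its owner a selectable RTS unit and tracks that unit's state.
; On BeginPlay it binds to the owner's click event; a click adds the owner to PC_RTSGame's selection and reveals the owner's DecalComponent.
; HandleNewUnitState stores the new state and calls the matching enter event for Idle, Movement or Mining.
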(event Custom|OnOwnerClicked
  (params (TouchedActor :type Actor%20Object%20Reference) (ButtonPressed :type Key%20Structure :default "None"))
  (CallFunction|AddUnitSelectionList)
  (CallFunction|ShowSelectedDecal))

(event Custom|ShowSelectedDecal
  (bind _returnvalue (Components|GetOwner))
  (bind _returnvalue_2 (Actor|GetComponentbyClass _returnvalue "/Script/Engine.DecalComponent"))
  (Rendering|SetVisibility _returnvalue_2 true false)
  (Development|SetHiddeninGame _returnvalue_2 false false))

(event Custom|AddUnitSelectionList
  (bind _aspc_rtsgame (Utilities|Casting|CastToPC_RTSGame (Game|GetPlayerController 0)))
  (Default|AddActorSelected _aspc_rtsgame (Components|GetOwner)))

(event EventBeginPlay
  (EventDispatchers|BindEventtoOnClicked (Components|GetOwner) (EventDispatchers|CreateEvent :!event Custom|OnOwnerClicked)))

(event EventTick
  (params (DeltaSeconds :type Float%20%28single-precision%29)))

(fn HandleNewUnitState
  (params (NewUnitState :type E_UnitStates%20Enum :default "NewEnumerator0"))
  (bind _output_get (Variables|Default|SetUnitState NewUnitState))
  (switch Utilities|FlowControl|Switch|SwitchonE_UnitStates _output_get
    (:NewEnumerator1
      (Default|CallOnEnterIdle))
    (:NewEnumerator2
      (Default|CallOneEnterMovement))
    (:NewEnumerator3
      (Default|CallOnEnterMining))))