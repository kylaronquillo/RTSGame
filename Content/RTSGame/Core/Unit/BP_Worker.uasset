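; BP_Worker is the RTS worker unit that moves on command, gathers resources and deposits them at the town hall.
; BP_UnitComponent holds the unit state, and its enter events switch the looping dwarf idle, walk and hit animations.
; Gathering chains AI MoveTo, a timed mining delay and a deposit to the player controller, repeating while the resource remains minable.
; Interacting with a matching building deposits any carried load.
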(event OnEnterIdle(BP_UnitComponent)
  (Components|Animation|PlayAnimation (Variables|Character|GetMesh) "/Game/RTSGameAssets/Characters/DwarfGrunt/Import_Animation/Dwarf_Idle.Dwarf_Idle" true))

(event OneEnterMovement(BP_UnitComponent)
  (Components|Animation|PlayAnimation (Variables|Character|GetMesh) "/Game/RTSGameAssets/Characters/DwarfGrunt/Import_Animation/Dwarf_Walk_mixamo_com.Dwarf_Walk_mixamo_com" true))

(event OnEnterMining(BP_UnitComponent)
  (Components|Animation|PlayAnimation (Variables|Character|GetMesh) "/Game/RTSGameAssets/Characters/DwarfGrunt/Import_Animation/Dwarf_Hit.Dwarf_Hit" true))

(event Custom|GoToTownHallAndDepositResource
  (params (Resource%20Ref :type Actor%20Object%20Reference))
  ;[1 1 1] Go to townhall to put resource
  (Default|HandleNewUnitState (Variables|Default|GetBP_UnitComponent) "NewEnumerator2")
  (bind _asgm_rtsgame (Utilities|Casting|CastToGM_RTSGame (Game|GetGameMode)))
  (AI|AIMoveTo self "0, 0, 0" (Default|GetPlayerTownHall _asgm_rtsgame) 2e+02 true
    (:OnSuccess
      (Default|HandleNewUnitState (Variables|Default|GetBP_UnitComponent) "NewEnumerator1")
      (bind _aspc_rtsgame (Utilities|Casting|CastToPC_RTSGame (Game|GetPlayerController 0)))
      (Default|ReceiveResources _aspc_rtsgame (Variables|Default|GetResourceBeingCarried) (Variables|Default|GetAmountOfResource))
      (Variables|Default|SetResourceBeingCarried "NewEnumerator0")
      (Variables|Default|SetAmountOfResource 0)
      (Utilities|IsValid Resource%20Ref
        (:Is%20Valid
          (CallFunction|RepeattheMiningAction Resource%20Ref))))))

(event Custom|RepeatTheMiningAction
  (params (InputPin :type Actor%20Object%20Reference))
  (if (Default|CanThisResourcebeMined (Actor|GetComponentbyClass InputPin "/Game/RTSGame/Core/Resources/BP_ResourceComponent.BP_ResourceComponent_C"))
    (CallFunction|GatherThisResource InputPin)))

(event EventBeginPlay)

(event Collision|EventActorBeginOverlap
  (params (OtherActor :type Actor%20Object%20Reference)))

(event EventTick
  (params (DeltaSeconds :type Float%20%28single-precision%29)))

(event EventInteractwithBuilding
  (params (Building%20Ref :type Actor%20Object%20Reference))
  (bind _returnvalue (Actor|GetComponentbyClass Building%20Ref "/Game/RTSGame/Core/Building/BP_BuildingComponent.BP_BuildingComponent_C"))
  (Utilities|IsValid _returnvalue
    (:Is%20Valid
      (if (> (Variables|Default|GetAmountOfResource) 0)
        (if (Utilities|Enum|Equal(Enum) (Variables|/Game/RTSGame/Core/Building/BP_BuildingComponent.BP_BuildingComponent_C|GetTypeOfBuilding _returnvalue) "NewEnumerator1")
          (CallFunction|GotoTownHallandDepositResource))))))

(event EventMovetoThisLocation
  (params (GoalLocation :type Vector :default "0, 0, 0"))
  (Default|HandleNewUnitState (Variables|Default|GetBP_UnitComponent) "NewEnumerator2")
  (bind _movementresult (AI|AIMoveTo self GoalLocation 0 5e+01 false)
    (:OnSuccess
      _)
    (:OnFail
      (switch Utilities|FlowControl|Switch|SwitchonEPathFollowingResult _movementresult
        (:Blocked
          _)
        (:OffPath
          _)
        (:Invalid
          _))))
  (Default|HandleNewUnitState (Variables|Default|GetBP_UnitComponent) "NewEnumerator1"))

(event EventGatherThisResource
  (params (ResourceReference :type Actor%20Object%20Reference))
  (bind _returnvalue (Actor|GetComponentbyClass ResourceReference "/Game/RTSGame/Core/Resources/BP_ResourceComponent.BP_ResourceComponent_C"))
  ;[1 1 1] Move to the resource and turn towards it
  (Default|HandleNewUnitState (Variables|Default|GetBP_UnitComponent) "NewEnumerator2")
  (AI|AIMoveTo self "0, 0, 0" ResourceReference 2e+02 false
    (:OnSuccess
      (Transformation|SetActorRotation (Math|Rotator|MakeRotator 0.0 0.0 (.yaw (Math|Rotator|FindLookatRotation (Transformation|GetActorLocation) (Transformation|GetActorLocation ResourceReference)))))
      ;[1 1 1] Start gathering the resource
      (if (and (Utilities|Enum|NotEqual(Enum) (Variables|Default|GetResourceBeingCarried) (Variables|/Game/RTSGame/Core/Resources/BP_ResourceComponent.BP_ResourceComponent_C|GetTypeOfResource _returnvalue)) (Default|CanThisResourcebeMined _returnvalue))
        (Default|HandleNewUnitState (Variables|Default|GetBP_UnitComponent) "NewEnumerator3")
        (Variables|Default|SetAmountOfResource 0)
        (Utilities|FlowControl|RetriggerableDelay (Variables|/Game/RTSGame/Core/Resources/BP_ResourceComponent.BP_ResourceComponent_C|GetTimeItTakesToBeGatheredS _returnvalue))
        ;[1 1 1] Getting thre Resource
        (if (Utilities|Enum|Equal(Enum) (Variables|/Game/RTSGame/Core/Unit/BP_UnitComponent.BP_UnitComponent_C|GetUnitState (Variables|Default|GetBP_UnitComponent)) "NewEnumerator3")
          (bind (_typeofresource _numofresourcestogive) (Default|GiveResource _returnvalue))
          (Variables|Default|SetResourceBeingCarried _typeofresource)
          (Variables|Default|SetAmountOfResource _numofresourcestogive)
          (CallFunction|GotoTownHallandDepositResource ResourceReference))
        (elif (and (Utilities|Enum|Equal(Enum) (Variables|Default|GetResourceBeingCarried) (Variables|/Game/RTSGame/Core/Resources/BP_ResourceComponent.BP_ResourceComponent_C|GetTypeOfResource _returnvalue)) (> (Variables|Default|GetAmountOfResource) 0))
          (CallFunction|GotoTownHallandDepositResource ResourceReference)
          (else
            (Default|HandleNewUnitState (Variables|Default|GetBP_UnitComponent) "NewEnumerator1")))))))

(event EventSelectThis
  (Default|ShowSelectedDecal (Variables|Default|GetBP_UnitComponent)))

(fn ConstructionScript)